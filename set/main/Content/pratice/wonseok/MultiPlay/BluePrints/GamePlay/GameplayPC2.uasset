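; GameplayPC2 is the multiplayer gameplay player controller, handling character spawning and chat.
; On BeginPlay the local controller clears widgets, loads player settings from a save game and passes them toward the server.
; That event asks GameplayGM2 to respawn the chosen character, then creates the chat widget.
; Chat messages fan out through the game mode's controller list to update each chat window, and T toggles the mouse cursor.
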(event `self.ReceiveBeginPlay`
  ;[1 1 1] 플레이어 정보를 불러와 서버상 플레이어 컨트롤러에 넘겨줌
  (if (`self.IsLocalController`)
    (`WidgetLayoutLibrary.RemoveAllWidgets`)
    (`self.LoadGame`)
    (`self.PassCharacterInfoToServer` (`self.PlayerSettings`))))

(event `PassCharacterInfoToServer`
  (params (PlayerSettingsInfo :type "/Game/pratice/wonseok/MultiPlay/BluePrints/AllLevels/PlayerInfo Structure"))
  ;[1 1 1] 캐릭터 정보 전송/ 플레이어가 선택한 플레이어를 스폰함 / ㅊ채팅창 구성 호출
  (set `self.PlayerSettings` PlayerSettingsInfo)
  (bind _asgameplay_gm2 (cast `/Game/pratice/wonseok/MultiPlay/BluePrints/GamePlay/GameplayGM2` (`GameplayStatics.GetGameMode`)))
  (`/Game/pratice/wonseok/MultiPlay/BluePrints/GamePlay/GameplayGM2.RespawnPlayer` _asgameplay_gm2 self (`.MyPlayerCharacter_11_B8C026C34D95289F75E145B8AE777C69` (break `/Game/pratice/wonseok/MultiPlay/BluePrints/AllLevels/PlayerInfo` (`self.PlayerSettings`))))
  (`self.SetupChatWindow`))

(event `SetupChatWindow`
  ;[1 1 1] 게임 플레이 내의 채팅창을 만들고 뷰포트에 추가함
  (bind _returnvalue (`|CreateWidget` "/Game/pratice/wonseok/MultiPlay/UI/AllLevels/GameplayChat.GameplayChat_C"))
  (bind _output_get (set `self.GameplayChatWB` _returnvalue))
  (`UserWidget.AddToViewport` _output_get 0))

(event `GetChatMessage`
  (params (TextToSend :type Text))
  ;[1 1 1] 채팅 입력 처리 / 클라이언트들에게 채팅을 업데이트하라고 통보
  (set `self.SenderText` TextToSend)
  (set `self.SenderName` (`.MyPlayerName_6_BD73401049AC67AF018D56A0843C3DBB` (break `/Game/pratice/wonseok/MultiPlay/BluePrints/AllLevels/PlayerInfo` (`self.PlayerSettings`))))
  (bind _asgameplay_gm2 (cast `/Game/pratice/wonseok/MultiPlay/BluePrints/GamePlay/GameplayGM2` (`GameplayStatics.GetGameMode`)))
  (for _array_element (`/Game/pratice/wonseok/MultiPlay/BluePrints/GamePlay/GameplayGM2.AllPlayerControllers` _asgameplay_gm2)
    (bind _asgameplay_pc2 (cast `/Game/pratice/wonseok/MultiPlay/BluePrints/GamePlay/GameplayPC2` _array_element))
    (`self.UpdateChat` _asgameplay_pc2 (`self.SenderName`) (`self.SenderText`))))

(event `UpdateChat`
  (params (SenderName :type Text) (SenderText :type Text))
  ;[1 1 1] 클라이언트의 채팅창을 업데이트
  (`/Game/pratice/wonseok/MultiPlay/UI/AllLevels/ChatWindow1.UpdateChatWindow` (`/Game/pratice/wonseok/MultiPlay/UI/AllLevels/GameplayChat.GameplayChat` (`self.GameplayChatWB`)) SenderName SenderText))

(event `Key|T`
  (params (Key :type "Key Structure"))
  ;[1 1 1] T키를 누르면 마우스 커서가 나타남
  (:`Pressed`
    (`/Engine/EditorBlueprintResources/StandardMacros.FlipFlop`
      (:`A`
        (set `self.bShowMouseCursor` true))
      (:`B`
        (set `self.bShowMouseCursor` false)))))

(fn `LoadGame`
  (bind _returnvalue (`GameplayStatics.LoadGameFromSlot` (`self.PlayerSettingSave`)))
  (bind _asplayer_save_game_1 (cast `/Game/pratice/wonseok/MultiPlay/BluePrints/AllLevels/PlayerSaveGame1` _returnvalue))
  (bind (_myplayername _myplayerimage _myplayercharacter) (break `/Game/pratice/wonseok/MultiPlay/BluePrints/AllLevels/PlayerInfo` (`/Game/pratice/wonseok/MultiPlay/BluePrints/AllLevels/PlayerSaveGame1.S_PlayerInfo` _asplayer_save_game_1)))
  (setmembers `/Game/pratice/wonseok/MultiPlay/BluePrints/AllLevels/PlayerInfo` :`StructRef` (`self.PlayerSettings`) :`MyPlayerName` _myplayername :`MyPlayerImage` _myplayerimage :`MyPlayerCharacter` _myplayercharacter :`MyPlayerCharacterImage` null :`MyPlaterStatus` "Not Ready!"))

(fn `UserConstructionScript`)