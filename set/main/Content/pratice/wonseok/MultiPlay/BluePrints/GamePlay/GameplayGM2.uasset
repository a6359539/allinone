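; Multiplayer gameplay game mode that tracks player controllers, respawns players and handles logout.
; Controllers arriving through OnSwapPlayerControllers are added to a list.
; RespawnPlayer destroys any current pawn, spawns Base at a random PlayerStart and possesses it, leaving its PlayerCharacter input unused despite the comment about selected characters.
; On logout, a GameplayPC2 controller is passed to the GameInstance to destroy its session.
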(event `self.K2_OnSwapPlayerControllers`
  (params (OldPC :type "PlayerController Object Reference") (NewPC :type "PlayerController Object Reference"))
  ;[1 1 1] 서버 접속자의 플레이어 컨트롤러 추적
  (`KismetArrayLibrary.Array_Add` (`self.AllPlayerControllers`) NewPC))

(event `RespawnPlayer`
  (params (PlayerController :type "PlayerController Object Reference") (PlayerCharacter :type "Character Class Reference"))
  (bind _returnvalue (`Controller.K2_GetPawn` PlayerController))
  (bind _spawnpoints (`self.SpawnPoints`))
  ;[1 1 1] 선택한 캐릭터를 게임플레이 컨트롤러에서 받아 스폰시켜줌
  (bind _outactors (`GameplayStatics.GetAllActorsOfClass` "/Script/Engine.PlayerStart"))
  (set `self.SpawnPoints` _outactors)
  (`/Engine/EditorBlueprintResources/StandardMacros.IsValid` _returnvalue
    (:`Is Valid`
      (`self.K2_DestroyActor` _returnvalue))
    (:`Is Not Valid`
      _))
  (bind _returnvalue_2 (`|SpawnActorFromClass` "/Game/pratice/wonseok/MultiPlay/BluePrints/Character/Base.Base_C" (`self.GetTransform` (`|GetArrayItem` _spawnpoints (`KismetMathLibrary.RandomIntegerInRange` 0 (- (`KismetArrayLibrary.Array_Length` _spawnpoints) 1)))) "Undefined" "OverrideRootScale" null null))
  (`Controller.Possess` PlayerController _returnvalue_2))

(event `self.K2_OnLogout`
  (params (ExitingController :type "Controller Object Reference"))
  ;[1 1 1] 로그아웃시 이벤트 발동 - Game Info Instance 에서 세션 파기 호출
  (bind _asgameplay_pc2 (cast `/Game/pratice/wonseok/MultiPlay/BluePrints/GamePlay/GameplayPC2` ExitingController))
  (`/Game/pratice/wonseok/MultiPlay/BluePrints/AllLevels/GameInstance.DestroySessionCaller` (cast `/Game/pratice/wonseok/MultiPlay/BluePrints/AllLevels/GameInstance` (`GameplayStatics.GetGameInstance`) :!pure true) _asgameplay_pc2))

(fn `UserConstructionScript`)