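; Multiplayer trap actor that explodes shortly after something overlaps its sphere.
; The server sets Armed on overlap, and its RepNotify starts a short fuse timer.
; When the fuse expires, only the server damages pawns within a radius and calls OnExplosion.
; OnExplosion plays the particle and sound, hides the actor and disables collision, while the server sets a short lifespan for cleanup.
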(event `self.Sphere.OnComponentBeginOverlap`
  (params (OverlappedComponent :type "PrimitiveComponent Object Reference") (OtherActor :type "Actor Object Reference") (OtherComp :type "PrimitiveComponent Object Reference") (OtherBodyIndex :type Integer) (bFromSweep :type Boolean) (SweepResult :type "HitResult Structure (by ref)"))
  (`/Engine/EditorBlueprintResources/ActorMacros.Switch Has Authority`
    (:`Authority`
      (set `self.Armed` true))))

(event `OnExplosion`
  (bind _returnvalue (`KismetMathLibrary.MakeVector` (.x (`self.K2_GetActorLocation`)) (.y (`self.K2_GetActorLocation`)) (- (.z (`self.K2_GetActorLocation`)) 100.0)))
  (`GameplayStatics.SpawnEmitterAtLocation` "/Game/InfinityBladeEffects/Effects/FX_Mobile/Fire/combat/P_ProjectileLob_Explo_Fire_02.P_ProjectileLob_Explo_Fire_02" _returnvalue (struct) (2.0 2.0 2.0))
  (`GameplayStatics.PlaySoundAtLocation` "/Game/StarterContent/Audio/Explosion02.Explosion02" _returnvalue)
  (`self.SetActorEnableCollision` false)
  (`self.SetActorHiddenInGame` true))

(fn `ApplyExplosionDamage`
  (bind _outactors (`KismetSystemLibrary.SphereOverlapActors` (`self.K2_GetActorLocation`) 200.0 (`|MakeArray` "ObjectTypeQuery3" :!type "EObjectTypeQuery Enum")))
  (for _array_element _outactors
    (`GameplayStatics.ApplyDamage` _array_element 20.0 (`self.GetInstigatorController`) self)))

(fn `OnFuseExpired`
  (`/Engine/EditorBlueprintResources/ActorMacros.Switch Has Authority`
    (:`Authority`
      (if (`self.Armed`)
        (`self.ApplyExplosionDamage`)
        (`self.OnExplosion`)
        (`self.SetLifeSpan` 1.5)))))

(fn `OnRep_Armed`
  (if (`self.Armed`)
    (`KismetSystemLibrary.K2_SetTimer` null "OnFuseExpired" 1.5)))

(fn `UserConstructionScript`)