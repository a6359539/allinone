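; Rain arrow projectile actor that travels downward along its Sphere's local axis and damages what it hits.
; Tick sets its location directly by a fixed per-frame offset, without sweep or delta-time scaling.
; The first overlap runs a debug-drawn capsule trace ahead, applying damage and destroying the arrow on a hit.
; That check is one-shot even if the trace misses; projectile-stop and particle-spawn events are empty.
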(event `self.ReceiveBeginPlay`)

(event `self.ReceiveTick`
  (params (DeltaSeconds :type "Float (single-precision)"))
  (bind _returnvalue (+ (* (`SceneComponent.GetUpVector` (`self.Sphere`)) -50.0) (`self.location`)))
  (set `self.location` _returnvalue)
  (`self.K2_SetActorLocation` _returnvalue))

(event `self.ReceiveActorBeginOverlap`
  (params (OtherActor :type "Actor Object Reference"))
  (bind _sphere (`self.Sphere`))
  (bind _returnvalue (`SceneComponent.K2_GetComponentLocation` _sphere))
  (if (`self.DoOnce`)
    (set `self.DoOnce` false)
    (bind (_outhit _returnvalue_2) (`KismetSystemLibrary.CapsuleTraceSingle` :`Start` _returnvalue :`End` (+ (* (`SceneComponent.GetUpVector` _sphere) -30.0) _returnvalue) :`Radius` 30.0 :`TraceChannel` "TraceTypeQuery1" :`DrawDebugType` "ForDuration"))
    (if _returnvalue_2
      (`GameplayStatics.ApplyDamage` (`.HitActor` (`GameplayStatics.BreakHitResult` _outhit)) 20.0 (`self.GetInstigatorController`) self)
      (`self.K2_DestroyActor`))))

(event `self.ProjectileMovement.OnProjectileStop`
  (params (ImpactResult :type "HitResult Structure (by ref)")))

(event `self.ParticleSystem.OnParticleSpawn`
  (params (EventName :type Name) (EmitterTime :type "Float (single-precision)") (Location :type "Vector Structure") (Velocity :type "Vector Structure")))

(fn `UserConstructionScript`)