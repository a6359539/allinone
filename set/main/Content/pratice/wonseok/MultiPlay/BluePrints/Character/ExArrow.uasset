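; Explosive arrow projectile that pitches along its velocity each tick, with a custom event to scale its speed.
; On first overlap, a debug-drawn forward capsule trace finds the hit bone, attaches a StaticArrow there, explodes, damages the hit actor and destroys the arrow.
; When projectile movement stops by itself, it deals area damage to nearby pawns and plays the explosion effect and sound, without destroying itself.
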(event `self.ReceiveBeginPlay`)

(event `self.ReceiveTick`
  (params (DeltaSeconds :type "Float (single-precision)"))
  (`self.ArrowAngle`))

(event `hi`
  (params (NewParam :type "Float (double-precision)"))
  (bind _projectilemovement (`self.ProjectileMovement`))
  (set `MovementComponent.Velocity` (* (`MovementComponent.Velocity` _projectilemovement) NewParam) _projectilemovement))

(event `ArrowAngle`
  (`self.K2_SetActorRotation` (`KismetMathLibrary.MakeRotator` (.roll (`self.K2_GetActorRotation`)) (.pitch (`KismetMathLibrary.MakeRotFromX` (`self.GetVelocity`))) (.yaw (`self.K2_GetActorRotation`)))))

(event `self.ReceiveActorBeginOverlap`
  (params (OtherActor :type "Actor Object Reference"))
  (bind _sphere (`self.Sphere`))
  (bind _returnvalue (`SceneComponent.K2_GetComponentLocation` _sphere))
  (if (`self.DoOnce`)
    (set `self.DoOnce` false)
    (bind (_outhit _returnvalue_2) (`KismetSystemLibrary.CapsuleTraceSingle` :`Start` _returnvalue :`End` (+ (* (`KismetMathLibrary.GetForwardVector` (`SceneComponent.K2_GetComponentRotation` _sphere)) 200.0) _returnvalue) :`TraceChannel` "TraceTypeQuery1" :`DrawDebugType` "ForDuration"))
    (if _returnvalue_2
      (bind (_bblockinghit _binitialoverlap _time _distance _location _impactpoint _normal _impactnormal _physmat _hitactor _hitcomponent _hitbonename) (`GameplayStatics.BreakHitResult` _outhit))
      (if (not (== _hitbonename "hgfdh"))
        (`MovementComponent.StopMovementImmediately` (`self.ProjectileMovement`))
        (`self.K2_SetActorLocation` _impactpoint)
        (bind _returnvalue_3 (`|SpawnActorFromClass` "/Game/pratice/wonseok/character/weapon/bow/StaticArrow.StaticArrow_C" (`self.GetTransform` self) "AlwaysSpawn" "OverrideRootScale" null null))
        (`SceneComponent.K2_AttachToComponent` (`Actor.RootComponent` _returnvalue_3) _hitcomponent _hitbonename "KeepWorld" "KeepWorld" "KeepWorld" true)
        (`self.Explosion`)
        (`GameplayStatics.ApplyDamage` _hitactor 50.0 (`self.GetInstigatorController`) self)
        (`self.K2_DestroyActor`)))))

(event `self.ProjectileMovement.OnProjectileStop`
  (params (ImpactResult :type "HitResult Structure (by ref)"))
  (`|ExecutionSequence`
    (:`then_0`
      (bind _outactors (`KismetSystemLibrary.SphereOverlapActors` (`self.K2_GetActorLocation`) 400.0 (`|MakeArray` "ObjectTypeQuery3" :!type "EObjectTypeQuery Enum")))
      (for _array_element _outactors
        (`GameplayStatics.ApplyDamage` _array_element 50.0 (`self.GetInstigatorController`) self)))
    (:`then_1`
      (`self.Explosion`))))

(event `Explosion`
  (bind _returnvalue (`KismetMathLibrary.MakeVector` (.x (`self.K2_GetActorLocation`)) (.y (`self.K2_GetActorLocation`)) (.z (`self.K2_GetActorLocation`))))
  (`GameplayStatics.SpawnEmitterAtLocation` "/Game/InfinityBladeEffects/Effects/FX_Mobile/Fire/combat/P_ProjectileLob_Explo_Fire_02.P_ProjectileLob_Explo_Fire_02" _returnvalue (struct) (7.0 7.0 7.0))
  (`GameplayStatics.PlaySoundAtLocation` "/Game/StarterContent/Audio/Explosion02.Explosion02" _returnvalue))

(event `self.ParticleSystem.OnParticleSpawn`
  (params (EventName :type Name) (EmitterTime :type "Float (single-precision)") (Location :type "Vector Structure") (Velocity :type "Vector Structure")))

(fn `UserConstructionScript`)