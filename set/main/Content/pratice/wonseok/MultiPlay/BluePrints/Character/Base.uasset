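; Multiplayer-project character base Blueprint combining melee combat, archer skills, inventory input and Health/Mana stats.
; Left click, authority-only, chains montage combos for sword-and-shield or greatsword, with events handling weapon visibility, launches and camera shake.
; Keys fire charged arrows, spawn traps and shoot a cable hook.
; A stat map drives timer regeneration and timeline-animated bars, but its HUD setup is disconnected and timeline updates never call StatLerpTick.
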(event `/Game/pratice/actioninter.dropaction`
  (params (inactor :type "Actor Object Reference"))
  (`self.SetActorHiddenInGame` inactor false)
  (`self.SetActorEnableCollision` inactor true)
  (`self.K2_SetActorTransform` inactor (`SceneComponent.K2_GetComponentToWorld` (`self.dropLoc`)) false false))

(event `Key|F`
  (params (Key :type "Key Structure"))
  (:`Pressed`
    (if (< (`KismetArrayLibrary.Array_Length` (`/Game/pratice/gamehud.inventory` (`self.gamehudwidget`))) 5)
      (`self.pickupitem`))))

(event `Key|I`
  (params (Key :type "Key Structure"))
  (bind _gamehudwidget (`self.gamehudwidget`))
  (bind _gamehudwidget_2 (`self.gamehudwidget`))
  (bind _gamehudwidget_3 (`self.gamehudwidget`))
  (:`Pressed`
    (if (and (`/Game/pratice/gamehud.activateinventory` _gamehudwidget_2) (!= (`self.inventorydelay`) true))
      (`/Engine/EditorBlueprintResources/StandardMacros.FlipFlop`
        (:`A`
          (set `/Game/pratice/gamehud.inventoryvisible` "Visible" _gamehudwidget_2)
          (`self.enablemousecusor`)
          (`UserWidget.PlayAnimation` _gamehudwidget_3 (`/Game/pratice/gamehud.itemanim` _gamehudwidget_3) 0.0 1 "Forward" 1.0)
          (set `self.inventorydelay` true)
          (set `self.memuopen` true)
          (`KismetSystemLibrary.Delay` 0.2)
          (set `self.inventorydelay` false))
        (:`B`
          (set `self.inventorydelay` true)
          (`UserWidget.PlayAnimation` _gamehudwidget (`/Game/pratice/gamehud.itemanim` _gamehudwidget) 0.0 1 "Reverse" 1.0)
          (`KismetSystemLibrary.Delay` 1.0)
          (set `/Game/pratice/gamehud.inventoryvisible` "Hidden" _gamehudwidget_2)
          (`self.disablemouscusor`)
          (set `self.memuopen` false))))))

(event `self.ReceiveBeginPlay`)

(event `SetupStatRegenerations`
  ;[1 1 1] setup the timers for stats that features regenerations
  (bind _keys (`BlueprintMapLibrary.Map_Keys` (`self.Stats`)))
  (for _array_element _keys
    (bind _data (`self.GetStat` _array_element))
    (bind ((`HasRegernation?_27_F5A609BB4E7C730CC14553AF6D617CB2` _hasregernation_) (`Regintervall_32_4A8C894248B5881D8F2B6897A65376ED` _regintervall) (`RegFunctionName_38_6141795F4E34FC1A5B005ABBB62514CB` _regfunctionname)) (break `/Game/pratice/wonseok/structures/s_StatData` _data))
    (if _hasregernation_
      (bind _returnvalue (`KismetSystemLibrary.K2_SetTimer` self _regfunctionname _regintervall true))
      (bind _structout (setmembers `/Game/pratice/wonseok/structures/s_StatData` :`StructRef` _data :`RegenerationTimer` _returnvalue))
      (`self.SetStatValue` _array_element _structout)
      (`self.HandleRegeneration` _array_element))))

(event `Key|Add`
  (params (Key :type "Key Structure"))
  (:`Pressed`
    (`self.ModifyStat` "NewEnumerator2" 50)
    (`self.ModifyStat` "NewEnumerator1" 50)))

(event `Key|Subtract`
  (params (Key :type "Key Structure"))
  (:`Pressed`
    (`self.ModifyStat` "NewEnumerator2" -50)
    (`self.ModifyStat` "NewEnumerator1" -50)))

(event `LerpStatDisplay`
  (params (Stat :type "/Game/pratice/wonseok/character/E_Stats Enum" :default "NewEnumerator0") (LerpTime :type "Float (double-precision)") (`InPositive?` :type Boolean))
  (bind ((`MaxValue_12_F012406349D24F6D0F1050A1FCD9534B` _maxvalue) (`CurrentValue_15_5BB22FB84FFB4DC759D675BAC36A75FD` _currentvalue) (`DisplayedValue_17_BC6C17674646A0DBCB2E499C5EA62D2A` _displayedvalue) (`BarWidget_23_B37375284FEE4483EC342F88B4FBE6D4` _barwidget)) (break `/Game/pratice/wonseok/structures/s_StatData` (`self.GetStat` Stat)))
  (`self.OnStatLerpStart` Stat)
  (`BlueprintMapLibrary.Map_Add` (`self.StatsLerpData`) Stat (make `/Game/pratice/wonseok/structures/s_StatLerp` _displayedvalue (`KismetMathLibrary.Conv_IntToDouble` _currentvalue) `InPositive?`))
  (`MaterialInstanceDynamic.SetScalarParameterValue` (`/Game/pratice/wonseok/widzet/wonseokHUD.DynamicMaterial` _barwidget) (select `bool` `InPositive?` :`false` "PercentLeft" :`true` "PercentRight" :!type "Name") (/ (`KismetMathLibrary.Conv_IntToDouble` _currentvalue) (`KismetMathLibrary.Conv_IntToDouble` _maxvalue)))
  (`Widget.SetVisibility` (`/Game/pratice/wonseok/widzet/wonseokHUD.statsremovebar` _barwidget) "SelfHitTestInvisible")
  (`TimelineComponent.SetTimelineLength` (select `/Game/pratice/wonseok/character/E_Stats` Stat :`NewEnumerator1` (`self.HpTimeline`) :`NewEnumerator2` (`self.ManaTimeline`)) LerpTime)
  (switch `/Game/pratice/wonseok/character/E_Stats` Stat
    (:`NewEnumerator1`
      (`Timeline|HpTimeline` :!via `PlayFromStart`
        (:`Update`
          (`self.OnStatLerpStart` "NewEnumerator1"))
        (:`Finished`
          (`self.OnStatLerpEnd` "NewEnumerator1"))))
    (:`NewEnumerator2`
      (`Timeline|ManaTimeline` :!via `PlayFromStart`
        (:`Update`
          (`self.OnStatLerpStart` "NewEnumerator2"))
        (:`Finished`
          (`self.OnStatLerpEnd` "NewEnumerator2"))))))

(event `ComboReset`
  ;[1 1 1] 콤보리셋
  (set `self.IsAttacking?` false)
  (set `self.ChainAttack` false)
  (set `self.Combo` 1))

(event `camshake`
  ;[1 1 1] Camera Shake
  (`PlayerController.ClientStartCameraShake` :`self` (`GameplayStatics.GetPlayerController` 0) :`Shake` "/Game/pratice/wonseok/character/charCamShake.charCamShake_C" :`Scale` (`self.camshake1`)))

(event `Launcher`
  (bind _charactermovement (`self.CharacterMovement`))
  ;[1 1 1] 런치 캐릭터
  (set `CharacterMovementComponent.GroundFriction` 0.0 _charactermovement)
  (`self.LaunchCharacter` (+ (* (`self.GetActorForwardVector`) (`self.LaunchForce`)) (* (`self.GetActorUpVector`) 1.0)))
  (`KismetSystemLibrary.RetriggerableDelay` 0.25)
  (set `CharacterMovementComponent.GroundFriction` 8.0 _charactermovement))

(event `UpLunch`
  (bind _charactermovement (`self.CharacterMovement`))
  ;[1 1 1] 캐릭터 위로 발사
  (set `CharacterMovementComponent.GroundFriction` 0.0 _charactermovement)
  (`self.LaunchCharacter` (+ (* (`self.GetActorForwardVector`) (`self.LaunchForce`)) (* (`self.GetActorUpVector`) 1500.0)))
  (`KismetSystemLibrary.RetriggerableDelay` 0.25)
  (set `CharacterMovementComponent.GroundFriction` 10.0 _charactermovement))

(event `Key|LeftMouseButton`
  (params (Key :type "Key Structure"))
  (:`Pressed`
    (`/Engine/EditorBlueprintResources/ActorMacros.Switch Has Authority`
      (:`Authority`
        (if (`self.Switching`)
          _
          (elif (`self.IsAttacking?`)
            (set `self.ChainAttack` true)
            (else
              (set `self.IsAttacking?` true)
              (if (`self.GreatSwordMode`) :!label _label
                ;[1 1 1] 양손검 공격
                (switch `int` (`self.Combo`)
                  (:`1`
                    (set `self.Combo` 2)
                    (set `self.AttMontage` "/Game/pratice/wonseok/character/animation/greatsword/W_GS01.W_GS01")
                    (set `self.LaunchForce` 100.0)
                    (set `self.camshake1` 0.7))
                  (:`2`
                    (set `self.Combo` 3)
                    (set `self.AttMontage` "/Game/pratice/wonseok/character/animation/greatsword/W_GS02.W_GS02")
                    (set `self.LaunchForce` 100.0)
                    (set `self.camshake1` 0.8))
                  (:`3`
                    (set `self.Combo` 4)
                    (set `self.AttMontage` "/Game/pratice/wonseok/character/animation/greatsword/W_GS3.W_GS3")
                    (set `self.LaunchForce` 400.0)
                    (set `self.camshake1` 0.9))
                  (:`4`
                    (set `self.AttMontage` "/Game/pratice/wonseok/character/animation/greatsword/W_GS04.W_GS04")
                    (set `self.LaunchForce` 100.0)
                    (set `self.camshake1` 5.0)))
                (`self.PlayAnimMontage` (`self.AttMontage`))
                (else
                  ;[1 1 1] 한손검 공격
                  (switch `int` (`self.Combo`)
                    (:`1`
                      (set `self.Combo` 2)
                      (set `self.AttMontage` "/Game/pratice/wonseok/character/animation/W_Montage1.W_Montage1")
                      (set `self.LaunchForce` 200.0)
                      (set `self.camshake1` 0.7))
                    (:`2`
                      (set `self.Combo` 3)
                      (set `self.AttMontage` "/Game/pratice/wonseok/character/animation/W_Montage3.W_Montage3")
                      (set `self.LaunchForce` 300.0)
                      (set `self.camshake1` 0.8))
                    (:`3`
                      (set `self.AttMontage` "/Game/pratice/wonseok/character/animation/W_Montage2.W_Montage2")
                      (set `self.LaunchForce` 400.0)
                      (set `self.camshake1` 0.9)))
                  (`self.PlayAnimMontage` (`self.AttMontage`)))))))))))

(event `gravity`
  (bind _charactermovement (`self.CharacterMovement`))
  ;[1 1 1] 캐릭터 위로 발사
  (set `CharacterMovementComponent.GravityScale` 20.0 _charactermovement)
  (`KismetSystemLibrary.RetriggerableDelay` 0.25)
  (set `CharacterMovementComponent.GravityScale` 1.0 _charactermovement))

(event `SwitchingON`
  ;[1 1 1] 스위칭 모드
  (set `self.Switching` true)
  (set `CharacterMovementComponent.MaxWalkSpeed` 0.0 (`self.CharacterMovement`)))

(event `ChainCombo`
  (if (`self.ChainAttack`)
    (set `self.ChainAttack` false)
    (goto _label)))

(event `SheathSword`
  ;[1 1 1] HIDE
  (`SceneComponent.SetHiddenInGame` (`self.Sword`) true false)
  (`SceneComponent.SetHiddenInGame` (`self.Shield1`) true false)
  ;[1 1 1] SHOW
  (`SceneComponent.SetHiddenInGame` (`self.Sheath`) false false)
  (`SceneComponent.SetHiddenInGame` (`self.ShieldOFF`) false false))

(event `SwitchingOFF`
  (bind _charactermovement (`self.CharacterMovement`))
  ;[1 1 1] 스위칭 모드
  (if (`self.GreatSwordMode`)
    (set `CharacterMovementComponent.MaxWalkSpeed` 250.0 _charactermovement)
    (else
      (set `CharacterMovementComponent.MaxWalkSpeed` 600.0 _charactermovement)))
  (`KismetSystemLibrary.RetriggerableDelay` 2.0)
  (set `self.Switching` false))

(event `DrawGS`
  ;[1 1 1] HIDE
  (`SceneComponent.SetHiddenInGame` (`self.GreatSword`) true false)
  ;[1 1 1] SHOW
  (`SceneComponent.SetHiddenInGame` (`self.GreatSwordON`) false false)
  (set `self.GreatSwordMode` true))

(event `skill`
  (`GameplayStatics.SpawnEmitterAtLocation` "/Game/InfinityBladeEffects/Effects/FX_Mobile/ICE/combat/P_HeldCharge_Ice_00.P_HeldCharge_Ice_00" (+ (* (`self.GetActorForwardVector`) 500.0) (`self.K2_GetActorLocation`)) (`self.K2_GetActorRotation`)))

(event `SheathGS`
  ;[1 1 1] HIDE
  (`SceneComponent.SetHiddenInGame` (`self.GreatSwordON`) true false)
  ;[1 1 1] SHOW
  (`SceneComponent.SetHiddenInGame` (`self.GreatSword`) false false))

(event `DrawSword`
  ;[1 1 1] HIDE
  (`SceneComponent.SetHiddenInGame` (`self.ShieldOFF`) true false)
  (`SceneComponent.SetHiddenInGame` (`self.Sheath`) true false)
  ;[1 1 1] SHOW
  (`SceneComponent.SetHiddenInGame` (`self.Shield1`) false false)
  (`SceneComponent.SetHiddenInGame` (`self.Sword`) false false)
  (set `self.GreatSwordMode` false))

(event `Key|R`
  (params (Key :type "Key Structure"))
  ;[1 1 1] 스위칭 모드
  (:`Pressed`
    (if (and (`self.Switching`) (`self.ChainAttack`))
      _
      (elif (not (`self.Switching`))
        (`/Engine/EditorBlueprintResources/StandardMacros.FlipFlop`
          (:`A`
            (set `self.SwitchMode` true))
          (:`B`
            (set `self.SwitchMode` false)))))))

(event `afterlauncharrow`
  (`SceneComponent.SetHiddenInGame` (`self.handarrow`) true false))

(event `Beforelauncharrow`
  (`SceneComponent.SetHiddenInGame` (`self.handarrow`) false false))

(event `Key|One`
  (params (Key :type "Key Structure"))
  (bind _arrowmaxspeed (`self.ArrowMaxSpeed`))
  ;[1 1 1] 폭발샷 AND 트랩
  (:`Pressed`
    (set `self.AimMode` true)
    (set `self.HoldButton` true)
    (if (`self.HoldButton`) :!label _label_2
      (if (< _arrowmaxspeed 3000.0)
        (set `self.ArrowMaxSpeed` (+ _arrowmaxspeed 100.0))
        (`KismetSystemLibrary.PrintString` (`KismetStringLibrary.Conv_DoubleToString` _arrowmaxspeed))
        (`KismetSystemLibrary.Delay` 0.05)
        (goto _label_2))))
  (:`Released`
    (set `self.AimMode` false)
    (set `self.HoldButton` false)
    (`|ExecutionSequence`
      (:`then_0`
        (bind _returnvalue (`|SpawnActorFromClass` "/Game/pratice/wonseok/MultiPlay/BluePrints/Character/Arrowactor.Arrowactor_C" (`KismetMathLibrary.MakeTransform` (`SceneComponent.K2_GetComponentLocation` (`self.ArrowRotation`)) (`SceneComponent.K2_GetComponentRotation` (`self.Arrow1`))) "AdjustIfPossibleButDontSpawnIfColliding" "OverrideRootScale" null null)) ; Spawn projectile
        (bind _projectilemovement (`/Game/pratice/wonseok/MultiPlay/BluePrints/Character/Arrowactor.ProjectileMovement` _returnvalue))
        (set `MovementComponent.Velocity` (* (`MovementComponent.Velocity` _projectilemovement) (`self.ArrowMaxSpeed`)) _projectilemovement)
        (set `self.ArrowMaxSpeed` 0.0)))))

(event `Key|T`
  (params (Key :type "Key Structure"))
  (bind _arrowmaxspeed (`self.ArrowMaxSpeed`))
  ;[1 1 1] 궁수 기본공격 및 멀티샷
  (:`Pressed`
    (set `self.AimMode` true)
    (set `self.HoldButton` true)
    (if (`self.HoldButton`) :!label _label_3
      (if (< _arrowmaxspeed 3000.0)
        (set `self.ArrowMaxSpeed` (+ _arrowmaxspeed 100.0))
        (`KismetSystemLibrary.PrintString` (`KismetStringLibrary.Conv_DoubleToString` _arrowmaxspeed))
        (`KismetSystemLibrary.Delay` 0.05)
        (goto _label_3))))
  (:`Released`
    (set `self.AimMode` false)
    (set `self.HoldButton` false)
    (`|ExecutionSequence`
      (:`then_0`
        (bind _returnvalue (`|SpawnActorFromClass` "/Game/pratice/wonseok/MultiPlay/BluePrints/Character/Arrowactor.Arrowactor_C" (`KismetMathLibrary.MakeTransform` (`SceneComponent.K2_GetComponentLocation` (`self.ArrowRotation`)) (`SceneComponent.K2_GetComponentRotation` (`self.Arrow1`))) "AdjustIfPossibleButDontSpawnIfColliding" "OverrideRootScale" null null)) ; Spawn projectile
        (bind _projectilemovement (`/Game/pratice/wonseok/MultiPlay/BluePrints/Character/Arrowactor.ProjectileMovement` _returnvalue))
        (set `MovementComponent.Velocity` (* (`MovementComponent.Velocity` _projectilemovement) (`self.ArrowMaxSpeed`)) _projectilemovement)))))

(event `Key|Two`
  (params (Key :type "Key Structure"))
  ;[1 1 1] 폭발샷 AND 트랩
  (:`Pressed`
    (bind _returnvalue (`|SpawnActorFromClass` "/Game/pratice/wonseok/character/weapon/bow/trap.trap_C" (`KismetMathLibrary.MakeTransform` (+ (* (`self.GetActorForwardVector`) 400.0) (`SceneComponent.K2_GetComponentLocation` (`self.Mesh`)))) "Undefined" "OverrideRootScale" null null))
    (set `/Game/pratice/wonseok/character/weapon/bow/trap.fire?` true _returnvalue)))

(event `Key|Three`
  (params (Key :type "Key Structure"))
  (bind (_returnvalue_location _returnvalue_rotation) (`KismetMathLibrary.BreakTransform` (`SceneComponent.K2_GetComponentToWorld` (`self.GetParentComponent`))))
  (:`Pressed`
    (`/Engine/EditorBlueprintResources/StandardMacros.DoOnce` false :!label _label_4
      (:`Completed`
        (`self.PlayAnimMontage` (`GameplayStatics.GetPlayerCharacter` 0) "/Game/pratice/wonseok/character/animation/sword_and_shield_attack__4__Montage.sword_and_shield_attack__4__Montage" 1.0 "None")
        (bind _returnvalue (`|SpawnActorFromClass` "/Game/pratice/wonseok/character/weapon/BP_Hook.BP_Hook_C" (`KismetMathLibrary.MakeTransform` (`SceneComponent.K2_GetComponentLocation` (`self.ArrowRotation`)) (`SceneComponent.K2_GetComponentRotation` (`self.Arrow1`))) "AdjustIfPossibleButAlwaysSpawn" "OverrideRootScale" null null)) ; Spawn projectile
        (bind _returnvalue_2 (`AddComponent|NODE_AddCableComponent-0` :`RelativeTransform` (`KismetMathLibrary.MakeTransform` _returnvalue_location _returnvalue_rotation)))
        (bind _output_get (set `self.Cable` _returnvalue_2))
        (`CableComponent.SetAttachEndTo` _output_get _returnvalue "None" "None")))))

(event `resethook`
  (bind _cable (`self.Cable`))
  (`|ExecutionSequence`
    (:`then_0`
      (`/Engine/EditorBlueprintResources/StandardMacros.IsValid` _cable
        (:`Is Valid`
          (`ActorComponent.K2_DestroyComponent` _cable))))
    (:`then_1`
      (goto _label_4 :!via `Reset`))))

(event `hookevent`)

(fn `disablemouscusor`
  (bind _returnvalue (`GameplayStatics.GetPlayerController` 0))
  (`WidgetBlueprintLibrary.SetInputMode_GameOnly` _returnvalue)
  (set `PlayerController.bShowMouseCursor` false _returnvalue))

(fn `enablemousecusor`
  (bind _returnvalue (`GameplayStatics.GetPlayerController` 0))
  (`WidgetBlueprintLibrary.SetInputMode_GameAndUIEx` _returnvalue (`self.gamehudwidget`))
  (set `PlayerController.bShowMouseCursor` true _returnvalue))

(fn `GetStat`
  (params (Stat :type "/Game/pratice/wonseok/character/E_Stats Enum" :default "NewEnumerator0"))
  (returns (Data :type "/Game/pratice/wonseok/structures/s_StatData Structure"))
  (return (`BlueprintMapLibrary.Map_Find` (`self.Stats`) Stat)))

(fn `HandleRegeneration`
  (params (stat :type "/Game/pratice/wonseok/character/E_Stats Enum" :default "NewEnumerator0"))
  (bind ((`MaxValue_12_F012406349D24F6D0F1050A1FCD9534B` _maxvalue) (`CurrentValue_15_5BB22FB84FFB4DC759D675BAC36A75FD` _currentvalue) (`RegenerationTimer_36_EBA44F164E688F57410BB08FD1EFEE9D` _regenerationtimer)) (break `/Game/pratice/wonseok/structures/s_StatData` (`self.GetStat` stat)))
  (bind _returnvalue (`KismetSystemLibrary.K2_IsTimerPausedHandle` _regenerationtimer))
  (if (and _returnvalue (!= _currentvalue _maxvalue))
    (`KismetSystemLibrary.K2_UnPauseTimerHandle` _regenerationtimer)
    (return)
    (elif (and (not _returnvalue) (== _currentvalue _maxvalue))
      (`KismetSystemLibrary.K2_PauseTimerHandle` _regenerationtimer)
      (return)
      (else
        (return)))))

(fn `HealthRegenTick`
  (bind ((`MaxValue_12_F012406349D24F6D0F1050A1FCD9534B` _maxvalue) (`TimeToRegMaxValue_30_B9BCD6524DDD95F37CF37AB1877E90AF` _timetoregmaxvalue) (`Regintervall_32_4A8C894248B5881D8F2B6897A65376ED` _regintervall)) (break `/Game/pratice/wonseok/structures/s_StatData` (`self.GetStat` "NewEnumerator1")))
  (`self.ModifyStat` "NewEnumerator1" (`KismetMathLibrary.FTrunc` (* (`KismetMathLibrary.Conv_IntToDouble` _maxvalue) (/ _regintervall _timetoregmaxvalue))))
  (return))

(fn `ManaRegenTick`
  (bind ((`MaxValue_12_F012406349D24F6D0F1050A1FCD9534B` _maxvalue) (`TimeToRegMaxValue_30_B9BCD6524DDD95F37CF37AB1877E90AF` _timetoregmaxvalue) (`Regintervall_32_4A8C894248B5881D8F2B6897A65376ED` _regintervall)) (break `/Game/pratice/wonseok/structures/s_StatData` (`self.GetStat` "NewEnumerator2")))
  (`self.ModifyStat` "NewEnumerator2" (`KismetMathLibrary.FTrunc` (* (`KismetMathLibrary.Conv_IntToDouble` _maxvalue) (/ _regintervall _timetoregmaxvalue))))
  (return))

(fn `ModifyStat`
  (params (Stat :type "/Game/pratice/wonseok/character/E_Stats Enum" :default "NewEnumerator0") (By :type Integer) (`Animated?` :type Boolean))
  (locals (localStat :type "/Game/pratice/wonseok/character/E_Stats Enum" :default "NewEnumerator0") (localBy :type Integer) (localAnimated :type Boolean) (LocalLerpAlpha :type "Float (double-precision)" :default 0.0))
  (bind _localstat (`local.localStat`))
  (bind _localstat_2 (`local.localStat`))
  (bind _data (`self.GetStat` (`local.localStat`)))
  (bind ((`MinValue_10_0211C2254277521BA007109911B8C7B9` _minvalue) (`MaxValue_12_F012406349D24F6D0F1050A1FCD9534B` _maxvalue) (`CurrentValue_15_5BB22FB84FFB4DC759D675BAC36A75FD` _currentvalue)) (break `/Game/pratice/wonseok/structures/s_StatData` _data))
  (bind (_minvalue_2 _maxvalue_2 _currentvalue_2 _displayedvalue _minlerptime _maxlerptime) (break `/Game/pratice/wonseok/structures/s_StatData` (`self.GetStat` (`local.localStat`))))
  (bind _returnvalue (`KismetMathLibrary.Clamp` (+ _currentvalue (`local.localBy`)) _minvalue _maxvalue))
  (set `local.localStat` Stat)
  (set `local.localBy` By)
  (bind _output_get (set `local.localAnimated` `Animated?`))
  (if _output_get
    (set `local.LocalLerpAlpha` (/ (`KismetMathLibrary.Conv_IntToDouble` (`KismetMathLibrary.Abs_Int` (`KismetMathLibrary.Clamp` (`local.localBy`) (* _currentvalue_2 -1) (- _maxvalue_2 _currentvalue_2)))) (`KismetMathLibrary.Conv_IntToDouble` _maxvalue_2)))
    (bind _structout (setmembers `/Game/pratice/wonseok/structures/s_StatData` :`StructRef` (`self.GetStat` _localstat) :`CurrentValue` _returnvalue))
    (`self.SetStatValue` _localstat _structout)
    (`self.HandleRegeneration` _localstat)
    (`self.LerpStatDisplay` (`local.localStat`) (`KismetMathLibrary.Lerp` _minlerptime _maxlerptime (`local.LocalLerpAlpha`)) (> (`local.localBy`) 0))
    (return)
    (else
      (bind _structout_2 (setmembers `/Game/pratice/wonseok/structures/s_StatData` :`StructRef` _data :`CurrentValue` _returnvalue :`DisplayedValue` (`KismetMathLibrary.Conv_IntToDouble` _returnvalue)))
      (`self.SetStatValue` _localstat_2 _structout_2)
      (`self.HandleRegeneration` _localstat_2)
      (`self.UpdateStat` _localstat_2)
      (return))))

(fn `OnStatLerpEnd`
  (params (Stat :type "/Game/pratice/wonseok/character/E_Stats Enum" :default "NewEnumerator0"))
  (bind _data (`self.GetStat` Stat))
  (bind ((`CurrentValue_15_5BB22FB84FFB4DC759D675BAC36A75FD` _currentvalue) (`BarWidget_23_B37375284FEE4483EC342F88B4FBE6D4` _barwidget)) (break `/Game/pratice/wonseok/structures/s_StatData` _data))
  (bind _structout (setmembers `/Game/pratice/wonseok/structures/s_StatData` :`StructRef` _data :`DisplayedValue` (`KismetMathLibrary.Conv_IntToDouble` _currentvalue) :`CurrentlyAnimated?` false))
  (`self.SetStatValue` Stat _structout)
  (`Widget.SetVisibility` (`/Game/pratice/wonseok/widzet/wonseokHUD.statsremovebar` _barwidget) "Hidden")
  (return))

(fn `OnStatLerpStart`
  (params (Stat :type "/Game/pratice/wonseok/character/E_Stats Enum" :default "NewEnumerator0"))
  (bind _structout (setmembers `/Game/pratice/wonseok/structures/s_StatData` :`StructRef` (`self.GetStat` Stat) :`CurrentlyAnimated?` true))
  (`self.SetStatValue` Stat _structout)
  (return))

(fn `SetStatValue`
  (params (Stat :type "/Game/pratice/wonseok/character/E_Stats Enum" :default "NewEnumerator0") (NewValue :type "/Game/pratice/wonseok/structures/s_StatData Structure"))
  (`BlueprintMapLibrary.Map_Add` (`self.Stats`) Stat NewValue)
  (return))

(fn `SetupStatBar`
  (bind _mianhud (`self.MianHUD`))
  (bind _structout (setmembers `/Game/pratice/wonseok/structures/s_StatData` :`StructRef` (`self.GetStat` "NewEnumerator1") :`BarWidget` (`/Game/pratice/wonseok/widzet/MainHUD.HealthBar` _mianhud)))
  (`self.SetStatValue` "NewEnumerator1" _structout)
  (bind _structout_2 (setmembers `/Game/pratice/wonseok/structures/s_StatData` :`StructRef` (`self.GetStat` "NewEnumerator2") :`BarWidget` (`/Game/pratice/wonseok/widzet/MainHUD.manabar` _mianhud)))
  (`self.SetStatValue` "NewEnumerator2" _structout_2)
  (return))

(fn `StatLerpTick`
  (params (Stat :type "/Game/pratice/wonseok/character/E_Stats Enum" :default "NewEnumerator0"))
  (bind _data (`self.GetStat` Stat))
  (bind ((`MaxValue_12_F012406349D24F6D0F1050A1FCD9534B` _maxvalue) (`DisplayedValue_17_BC6C17674646A0DBCB2E499C5EA62D2A` _displayedvalue) (`BarWidget_23_B37375284FEE4483EC342F88B4FBE6D4` _barwidget)) (break `/Game/pratice/wonseok/structures/s_StatData` _data))
  (bind _returnvalue (select `/Game/pratice/wonseok/character/E_Stats` Stat :`NewEnumerator1` (`self.HpTimeline`) :`NewEnumerator2` (`self.ManaTimeline`)))
  (bind (_originalvalue _valuetolerpto _poistive_) (break `/Game/pratice/wonseok/structures/s_StatLerp` (`BlueprintMapLibrary.Map_Find` (`self.StatsLerpData`) Stat)))
  (bind _structout (setmembers `/Game/pratice/wonseok/structures/s_StatData` :`StructRef` _data :`DisplayedValue` (`KismetMathLibrary.Lerp` _originalvalue _valuetolerpto (/ (`TimelineComponent.GetPlaybackPosition` _returnvalue) (`TimelineComponent.GetTimelineLength` _returnvalue)))))
  (`self.SetStatValue` Stat _structout)
  (`MaterialInstanceDynamic.SetScalarParameterValue` (`/Game/pratice/wonseok/widzet/wonseokHUD.DynamicMaterial` _barwidget) (select `bool` _poistive_ :`false` "PercentRight" :`true` "PercentLeft" :!type "Name") (/ _displayedvalue (`KismetMathLibrary.Conv_IntToDouble` _maxvalue)))
  (`self.UpdateStat` Stat)
  (return))

(fn `UpdateStat`
  (params (Stat :type "/Game/pratice/wonseok/character/E_Stats Enum" :default "NewEnumerator0"))
  (bind ((`MaxValue_12_F012406349D24F6D0F1050A1FCD9534B` _maxvalue) (`DisplayedValue_17_BC6C17674646A0DBCB2E499C5EA62D2A` _displayedvalue) (`BarWidget_23_B37375284FEE4483EC342F88B4FBE6D4` _barwidget)) (break `/Game/pratice/wonseok/structures/s_StatData` (`self.GetStat` Stat)))
  (bind _statbar (`/Game/pratice/wonseok/widzet/wonseokHUD.statbar` _barwidget))
  (bind _returnvalue (`KismetMathLibrary.FClamp` (/ _displayedvalue (`KismetMathLibrary.Conv_IntToDouble` _maxvalue))))
  (`/Engine/EditorBlueprintResources/StandardMacros.IsValid` _barwidget
    (:`Is Valid`
      (`ProgressBar.SetPercent` _statbar _returnvalue)
      (`TextBlock.SetText` (`/Game/pratice/wonseok/widzet/wonseokHUD.StatText` _barwidget) (`|FormatText` "{Displayed} / {Maximum}" (`KismetTextLibrary.Conv_IntToText` (`KismetMathLibrary.FTrunc` _displayedvalue) false) (`KismetTextLibrary.Conv_IntToText` _maxvalue false)))
      (if (`|EnumEquality` Stat "NewEnumerator1")
        (`ProgressBar.SetFillColorAndOpacity` _statbar (`KismetMathLibrary.LinearColorLerpUsingHSV` (struct :`R` 1.0 :`A` 1.0) (`/Game/pratice/wonseok/widzet/wonseokHUD.BarColor` _barwidget) _returnvalue))
        (return)
        (else
          (return))))
    (:`Is Not Valid`
      (return))))

(fn `UserConstructionScript`)