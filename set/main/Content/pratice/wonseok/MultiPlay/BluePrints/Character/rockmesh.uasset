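; Rock projectile actor that flies toward a stored Startvector point and bursts on contact.
; Tick teleport-steps it 20 units per frame toward that point, with no sweep or delta-time scaling.
; Box overlap destroys the actor, then spawns explosion and shield-slam emitters at and below Startvector.
; Emitter cleanup sits behind a Delay after DestroyActor, so it likely never runs; the timed-destroy logic is unwired.
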(event `self.ReceiveTick`
  (params (DeltaSeconds :type "Float (single-precision)"))
  (bind _returnvalue (`self.K2_GetActorLocation`))
  (`self.K2_SetActorLocation` (+ (* (`KismetMathLibrary.Normal` (- (`self.startvector`) _returnvalue)) 20.0) _returnvalue)))

(event `self.ReceiveBeginPlay`)

(event `destroy`)

(event `self.Box.OnComponentBeginOverlap`
  (params (OverlappedComponent :type "PrimitiveComponent Object Reference") (OtherActor :type "Actor Object Reference") (OtherComp :type "PrimitiveComponent Object Reference") (OtherBodyIndex :type Integer) (bFromSweep :type Boolean) (SweepResult :type "HitResult Structure (by ref)"))
  (bind (_startvector_x _startvector_y _startvector_z) (`KismetMathLibrary.BreakVector` (`self.startvector`)))
  (`self.K2_DestroyActor`)
  (bind _returnvalue (`GameplayStatics.SpawnEmitterAtLocation` "/Game/InfinityBladeEffects/Effects/FX_Monsters/FX_Monster_Gruntling/Notifies/P_Death_backpack_expl_02.P_Death_backpack_expl_02" (`self.startvector`)))
  (bind _returnvalue_2 (`GameplayStatics.SpawnEmitterAtLocation` "/Game/InfinityBladeEffects/Effects/FX_Monsters/FX_Monster_Ausar/P_AU_ShieldSlam_AOE.P_AU_ShieldSlam_AOE" (`KismetMathLibrary.MakeVector` _startvector_x _startvector_y (- _startvector_z 100.0)) (struct)))
  (`KismetSystemLibrary.Delay` 2.0)
  (`ActorComponent.K2_DestroyComponent` _returnvalue)
  (`ActorComponent.K2_DestroyComponent` _returnvalue_2))

(fn `UserConstructionScript`)