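; TeArrow is an arrow projectile actor driven by a ProjectileMovement component.
; Each Tick, ArrowAngle sets its pitch from the current velocity direction while keeping roll and yaw, so the arrow tilts along its flight path.
; A custom event named hi scales the projectile's velocity by a given multiplier.
; The BeginPlay, overlap and projectile-stop events are empty, so this graph contains no hit handling.
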(event `self.ReceiveBeginPlay`)

(event `self.ReceiveTick`
  (params (DeltaSeconds :type "Float (single-precision)"))
  (`self.ArrowAngle`))

(event `hi`
  (params (NewParam :type "Float (double-precision)"))
  (bind _projectilemovement (`self.ProjectileMovement`))
  (set `MovementComponent.Velocity` (* (`MovementComponent.Velocity` _projectilemovement) NewParam) _projectilemovement))

(event `ArrowAngle`
  (`self.K2_SetActorRotation` (`KismetMathLibrary.MakeRotator` (.roll (`self.K2_GetActorRotation`)) (.pitch (`KismetMathLibrary.MakeRotFromX` (`self.GetVelocity`))) (.yaw (`self.K2_GetActorRotation`)))))

(event `self.ReceiveActorBeginOverlap`
  (params (OtherActor :type "Actor Object Reference")))

(event `self.ProjectileMovement.OnProjectileStop`
  (params (ImpactResult :type "HitResult Structure (by ref)")))

(fn `UserConstructionScript`)