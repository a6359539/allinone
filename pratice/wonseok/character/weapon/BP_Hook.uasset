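; BP_Hook is a hook projectile that flies out, retracts to its spawn point and drags back any mbpc character it hits.
; BeginPlay stores the sphere's location, then after a brief delay plays the ComeBack timeline, which zeroes projectile velocity and lerps the sphere home.
; A hit also plays ComeBack, while a second timeline lerps the character's capsule to that point.
; Either timeline finishing sets Finish, whose OnRep is empty, and destroys the actor.
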(event `self.ReceiveBeginPlay`
  (bind _returnvalue (`SceneComponent.K2_GetComponentLocation` (`self.Sphere`)))
  (bind _output_get (set `self.Location` _returnvalue))
  (`KismetSystemLibrary.Delay` 0.1)
  (bind (_direction `_새_트랙_0`) (`Timeline|ComeBack` :!label _label)
    (:`Update`
      (set `MovementComponent.Velocity` (0.0 0.0 0.0) (`self.ProjectileMovement`))
      (`SceneComponent.K2_SetWorldLocation` (`self.Sphere`) (`KismetMathLibrary.VLerp` _returnvalue _output_get `_새_트랙_0`) false false))
    (:`Finished`
      (set `self.finish` true)
      (`self.K2_DestroyActor`))))

(event `self.Sphere.OnComponentHit`
  (params (HitComponent :type "PrimitiveComponent Object Reference") (OtherActor :type "Actor Object Reference") (OtherComp :type "PrimitiveComponent Object Reference") (NormalImpulse :type "Vector Structure") (Hit :type "HitResult Structure (by ref)"))
  (`|ExecutionSequence`
    (:`then_0`
      (goto _label))
    (:`then_1`
      (bind _asmbpc (cast `/Game/pratice/wonseok/MultiPlay/BluePrints/Character/mbpc` OtherActor))
      (bind (_direction `_새_트랙_0`) (`Timeline|타임라인_0`)
        (:`Update`
          (bind _capsulecomponent (`Character.CapsuleComponent` _asmbpc))
          (`SceneComponent.K2_SetWorldLocation` _capsulecomponent (`KismetMathLibrary.VLerp` (`SceneComponent.K2_GetComponentLocation` _capsulecomponent) (`self.Location`) `_새_트랙_0`) false false))
        (:`Finished`
          (set `self.finish` true)
          (`self.K2_DestroyActor`))))))

(fn `OnRep_finish`)

(fn `UserConstructionScript`)