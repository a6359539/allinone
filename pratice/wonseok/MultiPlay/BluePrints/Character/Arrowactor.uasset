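; Arrow projectile that pitches to follow its velocity each tick, with a custom event `hi` to scale its speed.
; On the first actor overlap only, it runs a debug-drawn capsule trace forward from its Sphere.
; A valid hit spawns a StaticArrow attached to the struck component and bone, applies damage and destroys the projectile.
; Particle effect and delayed-destroy nodes are left unconnected.
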(event `self.ReceiveBeginPlay`)

(event `self.ReceiveTick`
  (params (DeltaSeconds :type "Float (single-precision)"))
  (`self.ArrowAngle`))

(event `hi`
  (params (NewParam :type "Float (double-precision)"))
  (bind _projectilemovement (`self.ProjectileMovement`))
  (set `MovementComponent.Velocity` (* (`MovementComponent.Velocity` _projectilemovement) NewParam) _projectilemovement))

(event `ArrowAngle`
  (`self.K2_SetActorRotation` (`KismetMathLibrary.MakeRotator` (.roll (`self.K2_GetActorRotation`)) (.pitch (`KismetMathLibrary.MakeRotFromX` (`self.GetVelocity`))) (.yaw (`self.K2_GetActorRotation`)))))

(event `self.ReceiveActorBeginOverlap`
  (params (OtherActor :type "Actor Object Reference"))
  (bind _sphere (`self.Sphere`))
  (bind _returnvalue (`SceneComponent.K2_GetComponentLocation` _sphere))
  (if (`self.DoOnce`)
    (set `self.DoOnce` false)
    (bind (_outhit _returnvalue_2) (`KismetSystemLibrary.CapsuleTraceSingle` :`Start` _returnvalue :`End` (+ (* (`KismetMathLibrary.GetForwardVector` (`SceneComponent.K2_GetComponentRotation` _sphere)) 200.0) _returnvalue) :`TraceChannel` "TraceTypeQuery1" :`DrawDebugType` "ForDuration"))
    (if _returnvalue_2
      (bind (_bblockinghit _binitialoverlap _time _distance _location _impactpoint _normal _impactnormal _physmat _hitactor _hitcomponent _hitbonename) (`GameplayStatics.BreakHitResult` _outhit))
      (if (not (== _hitbonename "hgfdh"))
        (`MovementComponent.StopMovementImmediately` (`self.ProjectileMovement`))
        (`self.K2_SetActorLocation` _impactpoint)
        (bind _returnvalue_3 (`|SpawnActorFromClass` "/Game/pratice/wonseok/character/weapon/bow/StaticArrow.StaticArrow_C" (`self.GetTransform` self) "AlwaysSpawn" "OverrideRootScale" null null))
        (`SceneComponent.K2_AttachToComponent` (`Actor.RootComponent` _returnvalue_3) _hitcomponent _hitbonename "KeepWorld" "KeepWorld" "KeepWorld" true)
        (`GameplayStatics.ApplyDamage` _hitactor 20.0 (`self.GetInstigatorController`) self)
        (`self.K2_DestroyActor`)))))

(event `self.ProjectileMovement.OnProjectileStop`
  (params (ImpactResult :type "HitResult Structure (by ref)")))

(event `self.ParticleSystem.OnParticleSpawn`
  (params (EventName :type Name) (EmitterTime :type "Float (single-precision)") (Location :type "Vector Structure") (Velocity :type "Vector Structure")))

(fn `UserConstructionScript`)